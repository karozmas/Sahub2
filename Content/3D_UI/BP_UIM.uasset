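; BP_UIM is a 3D UI menu actor that moves the player's view to linked menu actors through its widget.
; On BeginPlay it binds to its WBP_Mean_3D widget and disables its own collision.
; An index received from the widget selects an actor from LMs, moving collision from this actor to the target and easing the first player's camera to it with SetViewTargetWithBlend.
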(event `self.ReceiveBeginPlay`
  (bind _aswbp_mean_3d (cast `/Game/3D_UI/Wigats/WBP_Mean_3D` (`WidgetComponent.GetUserWidgetObject` (`self.Widget`))))
  (add `/Game/3D_UI/Wigats/WBP_Mean_3D.TtoM` _aswbp_mean_3d (delegate `OnTBM`))
  (`self.SetActorEnableCollision` false))

(event `OnTBM`
  (params (Mindex :type Integer))
  (if (`KismetArrayLibrary.Array_IsValidIndex` (`self.LMs`) Mindex)
    (`self.TRTO` (`|GetArrayItem` (`self.LMs`) Mindex))))

(event `TRTO`
  (params (BP_UIM :type "/Game/3D_UI/BP_UIM Object Reference"))
  (`self.SetActorEnableCollision` false)
  (`self.SetActorEnableCollision` BP_UIM true)
  (`PlayerController.SetViewTargetWithBlend` (`GameplayStatics.GetPlayerController` 0) BP_UIM 2.0 "VTBlend_EaseInOut" 2.0 false))

(fn `UserConstructionScript`)