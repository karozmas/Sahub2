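; BP_Radiotap is a collectible radio tape pickup that counts toward the "FindTapes" task.
; A Box overlap enables player input on the actor and end overlap disables it, so F works only in range.
; Pressing F increments the task through ACTaskUpdater, then destroys the actor after a short delay.
; A separate event I calls the tape pickup message on Radio, with no caller in this graph.
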(event `Key|F`
  (params (Key :type "Key Structure"))
  (bind _ac_taskupdater (`self.AC_TaskUpdater`))
  (:`Pressed`
    (`/Game/SimpleTaskSystem/System/Blueprints/AC_TaskUpdater.Increment Task Progress` _ac_taskupdater (`/Game/SimpleTaskSystem/System/Blueprints/AC_TaskUpdater.Get Task ID By Name` _ac_taskupdater "FindTapes"))
    (`KismetSystemLibrary.Delay` 0.4)
    (`self.K2_DestroyActor`)))

(event `/Game/RadioS/BPI_I.I`
  (message `/Game/RadioS/BPI_P.Puk up Taep` (`self.Radio`)))

(event `self.Box.OnComponentBeginOverlap`
  (params (OverlappedComponent :type "PrimitiveComponent Object Reference") (OtherActor :type "Actor Object Reference") (OtherComp :type "PrimitiveComponent Object Reference") (OtherBodyIndex :type Integer) (bFromSweep :type Boolean) (SweepResult :type "HitResult Structure (by ref)"))
  (`self.EnableInput` (`GameplayStatics.GetPlayerController` 0)))

(event `self.Box.OnComponentEndOverlap`
  (params (OverlappedComponent :type "PrimitiveComponent Object Reference") (OtherActor :type "Actor Object Reference") (OtherComp :type "PrimitiveComponent Object Reference") (OtherBodyIndex :type Integer))
  (`self.DisableInput` (`GameplayStatics.GetPlayerController` 0)))

(fn `UserConstructionScript`)