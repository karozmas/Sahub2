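; BP_Radio2 is a radio actor that plays a 2D sound once it has been given a tape.
; Its box overlap enables player input and shows an input prompt widget while the first-person character is inside, undoing both on exit.
; The I key plays the sound only if the tape flag is set, which the PukUpTaep event turns on.
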(event `self.I`
  (if (`self.has teap?`)
    (`GameplayStatics.PlaySound2D` null 1.0 1.0 0.0 null null)))

(event `self.Puk up Taep`
  (set `self.has teap?` true))

(event `self.Box.OnComponentBeginOverlap`
  (params (OverlappedComponent :type "PrimitiveComponent Object Reference") (OtherActor :type "Actor Object Reference") (OtherComp :type "PrimitiveComponent Object Reference") (OtherBodyIndex :type Integer) (bFromSweep :type Boolean) (SweepResult :type "HitResult Structure (by ref)"))
  (cast `/Game/FirstPerson/Blueprints/BP_FirstPersonCharacter` OtherActor)
  (`self.EnableInput` (`GameplayStatics.GetPlayerController` 0))
  (bind _returnvalue (`|CreateWidget` "/Game/InputW/WBP_inputFandE.WBP_inputFandE_C"))
  (bind _output_get (set `self.NewVar` _returnvalue))
  (`UserWidget.AddToViewport` _output_get 0))

(event `self.Box.OnComponentEndOverlap`
  (params (OverlappedComponent :type "PrimitiveComponent Object Reference") (OtherActor :type "Actor Object Reference") (OtherComp :type "PrimitiveComponent Object Reference") (OtherBodyIndex :type Integer))
  (cast `/Game/FirstPerson/Blueprints/BP_FirstPersonCharacter` OtherActor)
  (`self.DisableInput` (`GameplayStatics.GetPlayerController` 0))
  (`Widget.RemoveFromParent` (`self.NewVar`)))

(fn `UserConstructionScript`)