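; Interactive GIS planting station that enables input and shows an F/T prompt while the first-person character is inside its Box trigger.
; Successive F presses step through a non-looping MultiGate of delayed Cube material swaps, then advance the "Use GIS In Bad Arae" task.
; T steps through two GIS widgets and then closes the last.
; A separate DroneArea trigger swaps the Cube material as BP_Drone enters and leaves.
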(event `self.Box.OnComponentBeginOverlap`
  (params (OverlappedComponent :type "PrimitiveComponent Object Reference") (OtherActor :type "Actor Object Reference") (OtherComp :type "PrimitiveComponent Object Reference") (OtherBodyIndex :type Integer) (bFromSweep :type Boolean) (SweepResult :type "HitResult Structure (by ref)"))
  (cast `/Game/FirstPerson/Blueprints/BP_FirstPersonCharacter` OtherActor)
  (`self.EnableInput` (`GameplayStatics.GetPlayerController` 0))
  (bind _returnvalue (`|CreateWidget` "/Game/InputW/WBP_inputFandT.WBP_inputFandT_C"))
  (bind _output_get (set `self.NewVar_1` _returnvalue))
  (`UserWidget.AddToViewport` _output_get 0))

(event `self.Box.OnComponentEndOverlap`
  (params (OverlappedComponent :type "PrimitiveComponent Object Reference") (OtherActor :type "Actor Object Reference") (OtherComp :type "PrimitiveComponent Object Reference") (OtherBodyIndex :type Integer))
  (cast `/Game/FirstPerson/Blueprints/BP_FirstPersonCharacter` OtherActor)
  (`self.DisableInput` (`GameplayStatics.GetPlayerController` 0))
  (`Widget.RemoveFromParent` (`self.NewVar_1`)))

(event `Key|F`
  (params (Key :type "Key Structure"))
  (bind _ac_taskupdater (`self.AC_TaskUpdater`))
  (:`Pressed`
    (`|MultiGate` false
      (:`Out 0`
        (`KismetSystemLibrary.Delay` 0.5)
        (`PrimitiveComponent.SetMaterial` (`self.Cube`) 0 "/Game/GIS/M_Pross.M_Pross"))
      (:`Out 1`
        (`KismetSystemLibrary.Delay` 0.5)
        (`PrimitiveComponent.SetMaterial` (`self.Cube`) 0 "/Game/Fab/Megascans/Surfaces/Arid_Gravel_Ground_wkjncjv/Medium/MI_wkjncjv.MI_wkjncjv"))
      (:`Out 2`
        (`KismetSystemLibrary.Delay` 0.5)
        (`PrimitiveComponent.SetMaterial` (`self.Cube`) 0 "/Game/GIS/M_Pross2.M_Pross2"))
      (:`Out 3`
        (`KismetSystemLibrary.Delay` 0.5)
        (`PrimitiveComponent.SetMaterial` (`self.Cube`) 0 "/Game/Fab/Megascans/Surfaces/Grass_And_Rubble_pjwey0/Medium/MI_pjwey0.MI_pjwey0"))
      (:`Out 4`
        (`KismetSystemLibrary.Delay` 1.0)
        (`/Game/SimpleTaskSystem/System/Blueprints/AC_TaskUpdater.Increment Task Progress` _ac_taskupdater (`/Game/SimpleTaskSystem/System/Blueprints/AC_TaskUpdater.Get Task ID By Name` _ac_taskupdater "Use GIS In Bad Arae"))))))

(event `self.DroneArea.OnComponentBeginOverlap`
  (params (OverlappedComponent :type "PrimitiveComponent Object Reference") (OtherActor :type "Actor Object Reference") (OtherComp :type "PrimitiveComponent Object Reference") (OtherBodyIndex :type Integer) (bFromSweep :type Boolean) (SweepResult :type "HitResult Structure (by ref)"))
  (cast `/Game/mydrone/BP_Drone` OtherActor)
  (`PrimitiveComponent.SetMaterial` (`self.Cube`) 0 "/Game/GIS/M_Pross3.M_Pross3"))

(event `self.DroneArea.OnComponentEndOverlap`
  (params (OverlappedComponent :type "PrimitiveComponent Object Reference") (OtherActor :type "Actor Object Reference") (OtherComp :type "PrimitiveComponent Object Reference") (OtherBodyIndex :type Integer))
  (cast `/Game/mydrone/BP_Drone` OtherActor)
  (`PrimitiveComponent.SetMaterial` (`self.Cube`) 0 "/Game/Fab/Megascans/Surfaces/Bright_Desert_Sand_sjzkfega/Medium/MI_sjzkfega.MI_sjzkfega"))

(event `Key|T`
  (params (Key :type "Key Structure"))
  (:`Pressed`
    (`|MultiGate` false
      (:`Out 0`
        (bind _returnvalue (`|CreateWidget` "/Game/GIS/W/WBP_GIS1.WBP_GIS1_C"))
        (bind _output_get (set `self.NewVar` _returnvalue))
        (`UserWidget.AddToViewport` _output_get 0))
      (:`Out 1`
        (`KismetSystemLibrary.Delay` 2.0)
        (`Widget.RemoveFromParent` (`self.NewVar`))
        (bind _returnvalue_2 (`|CreateWidget` "/Game/GIS/W/WBP_GIS2.WBP_GIS2_C"))
        (bind _output_get_2 (set `self.NewVar_0` _returnvalue_2))
        (`UserWidget.AddToViewport` _output_get_2 0))
      (:`Out 2`
        (`KismetSystemLibrary.Delay` 2.0)
        (`Widget.RemoveFromParent` (`self.NewVar_0`))))))

(fn `UserConstructionScript`)