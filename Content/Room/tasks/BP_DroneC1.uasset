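; BP_DroneC1 is an interactable task actor that the player collects to progress the "CollectTools" task.
; Entering its Box trigger enables input on player controller 0 and shows a WBP_inputF widget, and leaving disables input and removes it.
; Pressing F increments the task through ACTaskUpdater and destroys the actor.
; The overlap events do not filter which actor enters or leaves.
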(event `self.Box.OnComponentBeginOverlap`
  (params (OverlappedComponent :type "PrimitiveComponent Object Reference") (OtherActor :type "Actor Object Reference") (OtherComp :type "PrimitiveComponent Object Reference") (OtherBodyIndex :type Integer) (bFromSweep :type Boolean) (SweepResult :type "HitResult Structure (by ref)"))
  (`self.EnableInput` (`GameplayStatics.GetPlayerController` 0))
  (bind _returnvalue (`|CreateWidget` "/Game/InputW/WBP_inputF.WBP_inputF_C"))
  (bind _output_get (set `self.NewVar` _returnvalue))
  (`UserWidget.AddToViewport` _output_get 0))

(event `self.Box.OnComponentEndOverlap`
  (params (OverlappedComponent :type "PrimitiveComponent Object Reference") (OtherActor :type "Actor Object Reference") (OtherComp :type "PrimitiveComponent Object Reference") (OtherBodyIndex :type Integer))
  (`self.DisableInput` (`GameplayStatics.GetPlayerController` 0))
  (`Widget.RemoveFromParent` (`self.NewVar`)))

(event `Key|F`
  (params (Key :type "Key Structure"))
  (bind _ac_taskupdater (`self.AC_TaskUpdater`))
  (:`Pressed`
    (`/Game/SimpleTaskSystem/System/Blueprints/AC_TaskUpdater.Increment Task Progress` _ac_taskupdater (`/Game/SimpleTaskSystem/System/Blueprints/AC_TaskUpdater.Get Task ID By Name` _ac_taskupdater "CollectTools"))
    (`self.K2_DestroyActor`)))

(fn `UserConstructionScript`)