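; BP_TaskHandler is the gameplay-facing controller for an on-screen task list with progress counts.
; On BeginPlay it creates W_TaskWidget for player 0, adds it to the viewport and optionally hides the tasks.
; Its events and AddTask forward add, progress, finish, reset, visibility and removal calls to the widget, which holds the tasks.
; It binds the widget's completion dispatchers, re-broadcasts through its own, and resolves task names to array-index IDs.
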(event `ToggleTaskWidget`
  (bind _w_tasks_ref (`self.W_Tasks_REF`))
  (if (`Widget.IsVisible` (`self.W_Tasks_REF`))
    (`Widget.RemoveFromParent` _w_tasks_ref)
    (else
      (`UserWidget.AddToViewport` _w_tasks_ref 0))))

(event `self.ReceiveBeginPlay`
  ;[0 1 0.6719] Create Widget
  (bind _returnvalue (`|CreateWidget` "/Game/SimpleTaskSystem/System/Widgets/W_TaskWidget.W_TaskWidget_C" (`GameplayStatics.GetPlayerController` 0)))
  (bind _output_get (set `self.W_Tasks_REF` _returnvalue))
  (add `/Game/SimpleTaskSystem/System/Widgets/W_TaskWidget.On Specific Task Finished` _output_get (`|CreateDelegate` :!event `Internal On Task Finished`))
  (add `/Game/SimpleTaskSystem/System/Widgets/W_TaskWidget.On All Tasks Finished` _output_get (`|CreateDelegate` :!event `Internal On All Tasks Finished`))
  (`UserWidget.AddToViewport` _output_get 0)
  (if (`self.Start Hidden`)
    (`/Game/SimpleTaskSystem/System/Widgets/W_TaskWidget.Hide Tasks` _output_get)))

(event `Increment Task Progress`
  (params (TaskID :type Integer))
  ;[0.4766 0 1] Adds 1 to a tasks progress
  (`/Game/SimpleTaskSystem/System/Widgets/W_TaskWidget.Increment Task Progress` (`self.W_Tasks_REF`) TaskID))

(event `Decrement Task Progress`
  (params (`Task ID` :type Integer))
  ;[1 0.4688 0] Removes 1 from a tasks progress
  (`/Game/SimpleTaskSystem/System/Widgets/W_TaskWidget.Decrement Task Progress` (`self.W_Tasks_REF`) `Task ID`))

(event `Reset Task`
  (params (`Task ID` :type Integer))
  ;[1 0 0.07031] Resets a specific task to 0
  (`/Game/SimpleTaskSystem/System/Widgets/W_TaskWidget.Reset Task` (`self.W_Tasks_REF`) `Task ID`))

(event `Reset All Tasks`
  ;[0.05469 1 0] Resets all tasks to 0
  (`/Game/SimpleTaskSystem/System/Widgets/W_TaskWidget.Reset All Tasks` (`self.W_Tasks_REF`)))

(event `Finish Task`
  (params (`Task ID` :type Integer))
  ;[0.03125 1 0] Finishes a specific task
  (`/Game/SimpleTaskSystem/System/Widgets/W_TaskWidget.Finish Task` (`self.W_Tasks_REF`) `Task ID`))

(event `Finish All Tasks`
  ;[1 0.5859 0] Finishes all tasks
  (`/Game/SimpleTaskSystem/System/Widgets/W_TaskWidget.Finish All Tasks` (`self.W_Tasks_REF`)))

(event `Change All Tasks Max Count`
  (params (`Max Task Count` :type Integer))
  ;[0.1484 0 1] Change max count for all tasks
  (`/Game/SimpleTaskSystem/System/Widgets/W_TaskWidget.Change All Tasks Max Count` (`self.W_Tasks_REF`) `Max Task Count`))

(event `Change Task Max Count`
  (params (`Task ID` :type Integer) (`Max Task Count` :type Integer))
  ;[0 0.3672 1] Changes the maximum count of a task that needs to be completed
  (`/Game/SimpleTaskSystem/System/Widgets/W_TaskWidget.Change Task Max Count` (`self.W_Tasks_REF`) `Task ID` `Max Task Count`))

(event `Show Tasks`
  ;[1 0 0.5859] Makes all tasks visible
  (`/Game/SimpleTaskSystem/System/Widgets/W_TaskWidget.Show Tasks` (`self.W_Tasks_REF`)))

(event `Show Specific Task`
  (params (`Task ID` :type Integer))
  ;[1 0 0.9844] Makes a task visible when its hidden
  (`/Game/SimpleTaskSystem/System/Widgets/W_TaskWidget.Show Specific Task` (`self.W_Tasks_REF`) `Task ID`))

(event `Hide Specific Task`
  (params (`Task ID` :type Integer))
  ;[0 0.6953 1] Makes a task hidden when its visible
  (`/Game/SimpleTaskSystem/System/Widgets/W_TaskWidget.Hide Specific Task` (`self.W_Tasks_REF`) `Task ID`))

(event `Hide Tasks`
  ;[0 0.7891 1] Hides all tasks
  (`/Game/SimpleTaskSystem/System/Widgets/W_TaskWidget.Hide Tasks` (`self.W_Tasks_REF`)))

(event `Remove Specific Task`
  (params (`Task ID` :type Integer))
  ;[0 0.9766 1] Removes a specific tasks from the task list
  (`/Game/SimpleTaskSystem/System/Widgets/W_TaskWidget.Remove Specific Task` (`self.W_Tasks_REF`) `Task ID`))

(event `Remove All Tasks`
  ;[0.9688 0 1] Removes all tasks from the task list
  (`/Game/SimpleTaskSystem/System/Widgets/W_TaskWidget.Remove All Tasks` (`self.W_Tasks_REF`)))

(fn `Add Task`
  (params (TaskName :type Text) (`Initial Finished Count` :type Integer) (`Max Task Count` :type Integer))
  (returns (`Task ID` :type Integer))
  ;[0.3594 1 0] Adds a task to the screen
  (bind _task_id (`/Game/SimpleTaskSystem/System/Widgets/W_TaskWidget.Add Task` (`self.W_Tasks_REF`) TaskName `Initial Finished Count` `Max Task Count`))
  (return _task_id))

(fn `Get Task ID By Name`
  (params (`Task Name` :type Text))
  (returns (`Task ID` :type Integer))
  ;[0 1 0.3906] Get Task ID By Name
  (for (_array_element _array_index) (`/Game/SimpleTaskSystem/System/Widgets/W_TaskWidget.All Task Children` (`self.W_Tasks_REF`))
    (if (`KismetTextLibrary.EqualEqual_TextText` (`/Game/SimpleTaskSystem/System/Widgets/W_TaskChild.TaskName` _array_element) `Task Name`)
      (`|ExecutionSequence`
        (:`then_0`
          (break))
        (:`then_1`
          (return _array_index))))))

(fn `Internal On All Tasks Finished`
  (`self.On All Tasks Finished`))

(fn `Internal On Task Finished`
  (params (`Task ID` :type Integer) (`Task Name` :type Text))
  (`self.On Specific Task Finished` `Task ID` `Task Name`))

(fn `UserConstructionScript`)